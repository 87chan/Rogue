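; Player controller for the Rogue game that handles input for the skill selection window on the HUD.
; Holding OpenSkillWindow plays the skill widget's slide-in animation and releasing it plays the slide-out, tracked by an IsOpenSkillWindow flag.
; PrevIndex and NextIndex inputs step through the widget only while the window is open.
; CloseSkillWindowForce plays the out animation and clears the flag directly.
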(event `InputAction|OpenSkillWindow` :consume false
  (params (Key :type "Key Structure"))
  (bind _returnvalue (`self.GetHUD`))
  (bind _isopenskillwindow (`self.IsOpenSkillWindow`))
  (:`Pressed`
    (if (not _isopenskillwindow)
      (bind _asbp_hud (cast `/Game/Rogue/Blueprints/BP_HUD` _returnvalue))
      (bind _skillwidget (`/Game/Rogue/Blueprints/BP_HUD.SkillWidget` _asbp_hud))
      (`UserWidget.PlayAnimation` _skillwidget (`/Game/Rogue/Widgets/WBP_Skill.WindowIn` _skillwidget) 0.0 1 "Forward" 1.0)
      (set `self.IsOpenSkillWindow` true)))
  (:`Released`
    (if _isopenskillwindow
      (bind _asbp_hud_2 (cast `/Game/Rogue/Blueprints/BP_HUD` _returnvalue))
      (bind _skillwidget_2 (`/Game/Rogue/Blueprints/BP_HUD.SkillWidget` _asbp_hud_2))
      (`UserWidget.PlayAnimation` _skillwidget_2 (`/Game/Rogue/Widgets/WBP_Skill.WindowOut` _skillwidget_2) 0.0 1 "Forward" 1.0)
      (set `self.IsOpenSkillWindow` false))))

(event `InputAction|PrevIndex`
  (params (Key :type "Key Structure"))
  (:`Pressed`
    (if (`self.IsOpenSkillWindow`)
      (bind _asbp_hud (cast `/Game/Rogue/Blueprints/BP_HUD` (`self.GetHUD`)))
      (`/Game/Rogue/Widgets/WBP_Skill.PrevIndex` (`/Game/Rogue/Blueprints/BP_HUD.SkillWidget` _asbp_hud)))))

(event `InputAction|NextIndex`
  (params (Key :type "Key Structure"))
  (:`Pressed`
    (if (`self.IsOpenSkillWindow`)
      (bind _asbp_hud (cast `/Game/Rogue/Blueprints/BP_HUD` (`self.GetHUD`)))
      (`/Game/Rogue/Widgets/WBP_Skill.NextIndex` (`/Game/Rogue/Blueprints/BP_HUD.SkillWidget` _asbp_hud)))))

(fn `CloseSkillWindowForce`
  (bind _asbp_hud (cast `/Game/Rogue/Blueprints/BP_HUD` (`self.GetHUD`)))
  (bind _skillwidget (`/Game/Rogue/Blueprints/BP_HUD.SkillWidget` _asbp_hud))
  (`UserWidget.PlayAnimation` _skillwidget (`/Game/Rogue/Widgets/WBP_Skill.WindowOut` _skillwidget) 0.0 1 "Forward" 1.0)
  (set `self.IsOpenSkillWindow` false))

(fn `UserConstructionScript`)