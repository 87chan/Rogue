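; Base player pawn for a grid-based roguelike, moving one tile per directional key press and then advancing the game phase.
; Each move is validated by BP_MapManager, then offsets the root, turns the Cone mesh and updates the logical ArrayLocation before calling NextPhase.
; BeginPlay has the map manager create the map, places the player on a random cell and binds to the game mode's phase change, whose handler does nothing yet.
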(event `InputAction|MoveRight`
  (params (Key :type "Key Structure"))
  (bind _returnvalue (+ (`self.ArrayLocation`) (1.0 0.0)))
  (:`Pressed`
    (if (`MapManager.IsPossibleMove` (`self.MapManagerRef`) _returnvalue)
      (`SceneComponent.K2_AddLocalOffset` (`self.DefaultSceneRoot`) (0.0 100.0 0.0) false false)
      (`self.Turn` (`self.Cone`) "Dir_Right")
      (set `self.ArrayLocation` _returnvalue)
      (`/Game/Rogue/Blueprints/BP_FunctionLibrary.NextPhase` self :!label _label))))

(event `InputAction|MoveLeft`
  (params (Key :type "Key Structure"))
  (bind _returnvalue (+ (`self.ArrayLocation`) (-1.0 0.0)))
  (:`Pressed`
    (if (`MapManager.IsPossibleMove` (`self.MapManagerRef`) _returnvalue)
      (`SceneComponent.K2_AddLocalOffset` (`self.DefaultSceneRoot`) (0.0 -100.0 0.0) false false)
      (`self.Turn` (`self.Cone`) "Dir_Left")
      (set `self.ArrayLocation` _returnvalue)
      (goto _label))))

(event `InputAction|MoveForward`
  (params (Key :type "Key Structure"))
  (bind _returnvalue (+ (`self.ArrayLocation`) (0.0 -1.0)))
  (:`Pressed`
    (if (`MapManager.IsPossibleMove` (`self.MapManagerRef`) _returnvalue)
      (`SceneComponent.K2_AddLocalOffset` (`self.DefaultSceneRoot`) (100.0 0.0 0.0) false false)
      (`self.Turn` (`self.Cone`) "Dir_Upper")
      (set `self.ArrayLocation` _returnvalue)
      (goto _label))))

(event `InputAction|MoveBackward`
  (params (Key :type "Key Structure"))
  (bind _returnvalue (+ (`self.ArrayLocation`) (0.0 1.0)))
  (:`Pressed`
    (if (`MapManager.IsPossibleMove` (`self.MapManagerRef`) _returnvalue)
      (`SceneComponent.K2_AddLocalOffset` (`self.DefaultSceneRoot`) (-100.0 0.0 0.0) false false)
      (`self.Turn` (`self.Cone`) "Dir_Lower")
      (set `self.ArrayLocation` _returnvalue)
      (goto _label))))

(event `self.ReceiveBeginPlay`
  (`parent.ReceiveBeginPlay`)
  (`|ExecutionSequence`
    (:`then_0`
      (bind _outactors (`GameplayStatics.GetAllActorsOfClass` "/Game/Rogue/Blueprints/BP_MapManager.BP_MapManager_C"))
      (bind _output_get (set `self.MapManagerRef` (`|GetArrayItem` _outactors)))
      (`MapManager.CreateMap` _output_get))
    (:`then_1`
      (bind _output_get_2 (set `self.ArrayLocation` (`MapManager.GetRandomArrayLocation` (`self.MapManagerRef`))))
      (`self.AdjustLocation` _output_get_2)
      (`KismetSystemLibrary.PrintString` (`KismetTextLibrary.Conv_TextToString` (`|FormatText` "Place to : {0}" (`KismetTextLibrary.Conv_Vector2dToText` _output_get_2))) true true (struct :`G` 0.66 :`B` 1.0 :`A` 1.0) 500000.0))
    (:`then_2`
      (bind _asbp_game_mode_main (cast `/Game/Rogue/Blueprints/BP_GameMode_Main` (`GameplayStatics.GetGameMode`)))
      (add `RogueGameModeBase.OnPhaseChanged` _asbp_game_mode_main (delegate `OnPhaseChange`)))
    (:`then_3`
      (`self.Turn` (`self.Cone`) "Dir_Lower"))))

(event `OnPhaseChange`
  (params (PrevPhase :type "EPhaseType Enum" :default "Phase_PlayerAction") (NextPhase :type "EPhaseType Enum" :default "Phase_PlayerAction"))
  (switch `EPhaseType` NextPhase))

(fn `UserConstructionScript`)