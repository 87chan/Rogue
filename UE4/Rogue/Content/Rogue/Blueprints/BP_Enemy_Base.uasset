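; BP_Enemy_Base is the base enemy for a turn-based roguelike, acting in response to game phase changes.
; On BeginPlay it caches the map and enemy managers, registers itself, and binds to the game mode's phase-changed event.
; It takes damage during player attack, moves unless adjacent to the player during enemy move, and turns and attacks during enemy action.
; A ConsumeAction flag, reset each player action phase, gates that attack.
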(event `self.ReceiveBeginPlay`
  (`|ExecutionSequence`
    (:`then_0`
      (bind _outactors (`GameplayStatics.GetAllActorsOfClass` "/Game/Rogue/Blueprints/BP_MapManager.BP_MapManager_C"))
      (set `self.MapManager` (`|GetArrayItem` _outactors)))
    (:`then_1`
      (bind _outactors_2 (`GameplayStatics.GetAllActorsOfClass` "/Script/Rogue.EnemyManager"))
      (bind _output_get (set `self.EnemyManager` (`|GetArrayItem` _outactors_2)))
      (`EnemyManager.RegisterEnemy` _output_get self))
    (:`then_2`
      (add `RogueGameModeBase.OnPhaseChanged` (`/Game/Rogue/Blueprints/BP_MacroLibrary.BP_GameModeMain`) (delegate `OnPhaseChange`)))))

(event `OnPhaseChange`
  (params (PrevPhase :type "EPhaseType Enum" :default "Phase_PlayerAction") (NextPhase :type "EPhaseType Enum" :default "Phase_PlayerAction"))
  (switch `EPhaseType` NextPhase
    (:`Phase_PlayerAction`
      (set `self.bConsumeAction` false))
    (:`Phase_PlayerAttack`
      (set `self.ActivePhase` NextPhase)
      (`self.ApplyDamage` "Eff_PlayerAttack")
      (set `self.ActivePhase` "Phase_None")
      (`KismetSystemLibrary.PrintString` (`KismetStringLibrary.Conv_IntToString` (`self.LeftLifePoint`)) true true (struct :`R` 1.0 :`G` 0.005426 :`A` 1.0)))
    (:`Phase_EnemyMove`
      (set `self.ActivePhase` NextPhase)
      (if (not (`self.CheckAdjacent` "Fld_Player"))
        (`self.Move`))
      (set `self.ActivePhase` "Phase_None"))
    (:`Phase_EnemyAction`
      (set `self.ActivePhase` NextPhase)
      (if (not (`self.bConsumeAction`))
        (`self.TurnToPlayer`)
        (`self.Attack`))
      (set `self.ActivePhase` "Phase_None"))))

(fn `UserConstructionScript`)