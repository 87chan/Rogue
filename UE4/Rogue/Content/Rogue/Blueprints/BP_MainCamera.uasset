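; BP_MainCamera is a top-down camera actor that follows the player from overhead.
; On BeginPlay it makes itself the view target of the first player controller.
; Every tick it looks up all BP_Player_Base actors, takes the first as Target, and snaps to a point Distance units above it with a fixed rotation, without smoothing or a spring arm.
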(event `self.ReceiveBeginPlay`
  (`PlayerController.SetViewTargetWithBlend` (`GameplayStatics.GetPlayerController` 0) self 0.0 "VTBlend_Linear" 0.0 false))

(event `self.ReceiveTick`
  (params (DeltaSeconds :type "Float (single-precision)"))
  (`|ExecutionSequence`
    (:`then_0`
      (bind _outactors (`GameplayStatics.GetAllActorsOfClass` "/Game/Rogue/Blueprints/BP_Player_Base.BP_Player_Base_C"))
      (set `self.Target` (`|GetArrayItem` _outactors)))
    (:`then_1`
      (`self.K2_SetActorTransform` (`KismetMathLibrary.MakeTransform` (+ (`self.K2_GetActorLocation` (`self.Target`)) (* (0.0 0.0 1.0) (`self.Distance`))) (struct :`Pitch` -90.0))))))

(fn `UserConstructionScript`)